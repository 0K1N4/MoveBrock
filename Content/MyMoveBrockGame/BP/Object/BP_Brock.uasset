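; BP_Brock is a block that the player pushes along the world X or Y axis.
; OnhitPlayer checks lock, finish and facing state, then picks the axis and offset from the player pawn's forward vector.
; An X or Y timeline drives MoveBrock each update and calls ResetBrockPos when finished.
; A box overlap during movement sets a stop flag and registers the block as the third-person character's current interaction target.
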(event OnComponentBeginOverlap(BoxCol)
  (params (OverlappedComponent :type Primitive%20Component%20Object%20Reference) (OtherActor :type Actor%20Object%20Reference) (OtherComp :type Primitive%20Component%20Object%20Reference) (OtherBodyIndex :type Integer) (bFromSweep :type Boolean) (SweepResult :type Hit%20Result%20Structure%20%28by%20ref%29))
  ;[0 0.09648 1] プレイヤーとの接触判定
  (if (Variables|Default|Getm_bMove)
    (Variables|Default|Setm_bStop true)
    (bind _asbp_third_person_character (Utilities|Casting|CastToBP_ThirdPersonCharacter OtherActor))
    (Variables|/Game/ThirdPerson/Blueprints/BP_ThirdPersonCharacter.BP_ThirdPersonCharacter_C|SetCurrentIntaractTarget _asbp_third_person_character self)))

(event Custom|Event%20On%20hit%20Player
  (bind _returnvalue (Game|Player|GetPlayerPawn 0))
  (bind _returnvalue_2 (Transformation|GetActorForwardVector _returnvalue))
  (if (not (Variables|Default|Getm_bLock))
    (if (Variables|Default|Getm_bFinish)
      (bind _returnvalue_3 (Class|MyBrock|GetActorForwardVectortoObj _returnvalue))
      (if _returnvalue_3
        (bind _returnvalue_4 (Class|MyBrock|IsActorBiggerVec (.x _returnvalue_2) (.y _returnvalue_2)))
        (if _returnvalue_4
          ;[1 0.09896 0.09896 1 24] 移動
          (bind _returnvalue_5 (Class|MyBrock|GetMovementAmount (.x _returnvalue_2)))
          (bind _output_get (Variables|Default|Setm_fvOldVec (Math|Vector|MakeVector _returnvalue_5 0.0 0.0)))
          (Variables|Default|Setm_bMove true)
          (Timeline|XMove Play
            (:Update
              (Class|MyBrock|MoveBrock (Math|Vector|MakeVector (.x _output_get) 0.0 0.0)))
            (:Finished
              (Class|MyBrock|ResetBrockPos)))
          (else
            (bind _returnvalue_6 (Class|MyBrock|GetMovementAmount (.y _returnvalue_2)))
            (bind _output_get_2 (Variables|Default|Setm_fvOldVec (Math|Vector|MakeVector 0.0 _returnvalue_6 0.0)))
            (Variables|Default|Setm_bMove true)
            (Timeline|YMove Play
              (:Update
                (Class|MyBrock|MoveBrock (Math|Vector|MakeVector 0.0 (.y _output_get_2) 0.0)))
              (:Finished
                (Class|MyBrock|ResetBrockPos)))))))))

(event EventBeginPlay)

(event Collision|EventActorBeginOverlap
  (params (OtherActor :type Actor%20Object%20Reference)))

(event EventTick
  (params (DeltaSeconds :type Float%20%28single-precision%29)))

(fn ConstructionScript)